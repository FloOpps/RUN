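; Floor tile for an endless runner that randomly spawns either a collectible inside its area or a blocker at one of three spawn points on construction.
; Its end trigger asks RunGameMode to add another tile, then destroys this one a second later.
; Wall hits kill the RunCharacter when a dot-product test aligns hit normal with its forward vector.
; A distance box increments the runner's distance, and AttachPoint supplies the attach transform.
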(event `self.EndTriggerBox.OnComponentBeginOverlap`
  (params (OverlappedComponent :type "PrimitiveComponent Object Reference") (OtherActor :type "Actor Object Reference") (OtherComp :type "PrimitiveComponent Object Reference") (OtherBodyIndex :type Integer) (bFromSweep :type Boolean) (SweepResult :type "HitResult Structure (by ref)"))
  ;[1 1 1] Box to generate a new floor and destroy the previous one containing the EndTriggerBox hited
  (cast `/Game/ThirdPerson/Blueprints/RunCharacter` OtherActor)
  (bind _asrun_game_mode (cast `/Game/ThirdPerson/Blueprints/RunGameMode` (`GameplayStatics.GetGameMode`)))
  (`/Game/ThirdPerson/Blueprints/RunGameMode.AddFloorTile` _asrun_game_mode)
  (`KismetSystemLibrary.Delay` 1.0)
  (`self.K2_DestroyActor`))

(event `self.Wall.OnComponentHit`
  (params (HitComponent :type "PrimitiveComponent Object Reference") (OtherActor :type "Actor Object Reference") (OtherComp :type "PrimitiveComponent Object Reference") (NormalImpulse :type "Vector Structure") (Hit :type "HitResult Structure (by ref)"))
  ;[1 1 1] Death when the player hit a wall that is not in is direction
  (bind _asrun_character (cast `/Game/ThirdPerson/Blueprints/RunCharacter` OtherActor))
  (if (`KismetMathLibrary.NearlyEqual_FloatFloat` (`KismetMathLibrary.Dot_VectorVector` Hit_Normal (`self.GetActorForwardVector` _asrun_character)) 1.0 0.01)
    (`/Game/ThirdPerson/Blueprints/RunCharacter.Death` _asrun_character)))

(event `self.Wall1.OnComponentHit`
  (params (HitComponent :type "PrimitiveComponent Object Reference") (OtherActor :type "Actor Object Reference") (OtherComp :type "PrimitiveComponent Object Reference") (NormalImpulse :type "Vector Structure") (Hit :type "HitResult Structure (by ref)"))
  ;[1 1 1] Death when the player hit a wall that is not in is direction
  (bind _asrun_character (cast `/Game/ThirdPerson/Blueprints/RunCharacter` OtherActor))
  (if (`KismetMathLibrary.NearlyEqual_FloatFloat` (`KismetMathLibrary.Dot_VectorVector` Hit_Normal (`self.GetActorForwardVector` _asrun_character)) 1.0 0.01)
    (`/Game/ThirdPerson/Blueprints/RunCharacter.Death` _asrun_character)))

(event `self.BoxDistance.OnComponentBeginOverlap`
  (params (OverlappedComponent :type "PrimitiveComponent Object Reference") (OtherActor :type "Actor Object Reference") (OtherComp :type "PrimitiveComponent Object Reference") (OtherBodyIndex :type Integer) (bFromSweep :type Boolean) (SweepResult :type "HitResult Structure (by ref)"))
  (bind _asrun_character (cast `/Game/ThirdPerson/Blueprints/RunCharacter` OtherActor))
  (`/Game/ThirdPerson/Blueprints/RunCharacter.AddDistance` _asrun_character))

(fn `GetAttachTransform`
  (returns (AttachTransform :type "Transform Structure"))
  ;[1 1 1] Return the end of the position of the last floor spawned
  (return (`SceneComponent.K2_GetComponentToWorld` (`self.AttachPoint`))))

(fn `SetSpawnPoints`
  ;[1 1 1] get the position of all spawn point in the floor tile
  (set `self.SpawnPoints` (`|MakeArray` (`SceneComponent.GetRelativeTransform` (`self.SpawnPoint`)) (`SceneComponent.GetRelativeTransform` (`self.SpawnPointL`)) (`SceneComponent.GetRelativeTransform` (`self.SpawnPointR`)))))

(fn `SpawnBlocker`
  (bind _spawnpoints (`self.SpawnPoints`))
  ;[1 1 1] Spawn a blocker in a random position between all the possibility
  (`AddComponent|NODE_AddChildActorComponent-0` :`RelativeTransform` (`|GetArrayItem` _spawnpoints (`KismetMathLibrary.RandomIntegerInRange` 0 (`KismetArrayLibrary.Array_LastIndex` _spawnpoints)))))

(fn `SpawnCollect`
  (bind _collectarea (`self.CollectArea`))
  (`AddComponent|NODE_AddChildActorComponent-1` :`RelativeTransform` (`KismetMathLibrary.Conv_VectorToTransform` (`KismetMathLibrary.RandomPointInBoundingBox` (`SceneComponent.RelativeLocation` _collectarea) (`BoxComponent.BoxExtent` _collectarea)))))

(fn `UserConstructionScript`
  (`self.SetSpawnPoints`)
  (switch `int` (`KismetMathLibrary.RandomIntegerInRange` 0 1)
    (:`Default`
      (`self.SpawnCollect` :!label _label))
    (:`0`
      (goto _label))
    (:`1`
      (`self.SpawnBlocker`))))