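; BP_ramp_up is a floor tile for map generation, apparently an upward ramp, that places a blocker on itself.
; Its construction script gathers the relative transforms of three spawn point components into an array.
; It then adds a child actor component, the trap, at one randomly chosen transform.
; The event graph holds only disabled default events, so all logic runs at construction.
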(fn `Set Spawn Points`
  ;[1 1 1] get the position of all spawn point in the floor tile
  (set `self.SpawnPoints` (`|MakeArray` (`SceneComponent.GetRelativeTransform` (`self.SpawnPoint1`)) (`SceneComponent.GetRelativeTransform` (`self.SpawnPointL1`)) (`SceneComponent.GetRelativeTransform` (`self.SpawnPointR1`)))))

(fn `Spawn Trap`
  (bind _spawnpoints (`self.SpawnPoints`))
  ;[1 1 1] Spawn a blocker in a random position between all the possibility
  (`AddComponent|NODE_AddChildActorComponent-0` :`RelativeTransform` (`|GetArrayItem` _spawnpoints (`KismetMathLibrary.RandomIntegerInRange` 0 (`KismetArrayLibrary.Array_LastIndex` _spawnpoints)))))

(fn `UserConstructionScript`
  (`self.Set Spawn Points`)
  (`self.Spawn Trap`))